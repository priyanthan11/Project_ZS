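; Procedural map prototype actor that builds a vertex array and previews it with debug points.
; On BeginPlay, GenerateZS loops AreaHeightY on both axes, using 1D Perlin noise of each index over CellSize as X and Y, with Z at zero.
; An alternative GenerateMap lays out a flat width-by-height grid spaced by CellSize but is never called.
; The procedural mesh creation is also disconnected, so no mesh is built.
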(event `self.ReceiveBeginPlay`
  (`self.Generate ZS`))

(fn `Generate Map`
  (locals (aw_Y :type Integer) (aw_X :type Integer))
  (bind _vertices (`self.Vertices`))
  (for _index (range (`self.area_height_Y`))
    (set `local.aw_Y` _index)
    (for _index_2 (range (`self.area_width_X`))
      (set `local.aw_X` _index_2)
      (bind _returnvalue (`KismetArrayLibrary.Array_Add` _vertices (`KismetMathLibrary.MakeVector` (* _index_2 (`self.CellSize`)) (* (`local.aw_Y`) (`self.CellSize`)))))
      (bind (_output_x _output_y) (`KismetMathLibrary.BreakVector` (`|GetArrayItem` _vertices _returnvalue)))
      (`KismetSystemLibrary.DrawDebugPoint` (`KismetMathLibrary.MakeVector` _output_x _output_y) 5.0 (struct) 200.0))))

(fn `Generate ZS`
  (locals (X :type Integer) (Y :type Integer))
  (bind _vertices (`self.Vertices`))
  (for _index (range (`self.area_height_Y`))
    (set `local.X` _index)
    (for _index_2 (range (`self.area_height_Y`))
      (set `local.Y` _index_2)
      (bind _returnvalue (`KismetArrayLibrary.Array_Add` _vertices (`KismetMathLibrary.MakeVector` (`KismetMathLibrary.PerlinNoise1D` (/ (`local.X`) (`self.CellSize`))) (`KismetMathLibrary.PerlinNoise1D` (/ (`local.Y`) (`self.CellSize`))))))
      (bind (_output_x _output_y) (`KismetMathLibrary.BreakVector` (`|GetArrayItem` _vertices _returnvalue)))
      (`KismetSystemLibrary.DrawDebugPoint` (`KismetMathLibrary.MakeVector` _output_x _output_y) 5.0 (struct) 200.0))))

(fn `UserConstructionScript`)