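; Procedural terrain actor that builds a grid mesh with random vertex heights at BeginPlay; despite the DimandSq name, it runs no diamond-square pass.
; GenerateVerticies fills positions and UVs from the grid size and scale, drawing a long-lived debug sphere at each grid point.
; GenerateTriangle indexes two triangles per cell, then ProceduralMesh creates the section with collision and applies the material.
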(event `self.ReceiveBeginPlay`
  (`self.Generate Verticies`)
  (`self.Generate Triangle`)
  (`ProceduralMeshComponent.CreateMeshSection_LinearColor` :`self` (`self.ProceduralMesh`) :`Vertices` (`self.Vertices`) :`Triangles` (`self.Triangles`) :`UV0` (`self.UV0`) :`bCreateCollision` true)
  (`PrimitiveComponent.SetMaterial` (`self.ProceduralMesh`) 0 (`self.Material`)))

(fn `Generate Triangle`
  (locals (Vertext :type Integer))
  (for _ (range (`self.XSize`))
    (for _ (range (`self.YSize`))
      (`KismetArrayLibrary.Array_Add` (`self.Triangles`) (`local.Vertext`))
      (`KismetArrayLibrary.Array_Add` (`self.Triangles`) (+ (`local.Vertext`) 1))
      (`KismetArrayLibrary.Array_Add` (`self.Triangles`) (+ (`self.YSize`) 1 (`local.Vertext`)))
      (`KismetArrayLibrary.Array_Add` (`self.Triangles`) (+ (`local.Vertext`) 1))
      (`KismetArrayLibrary.Array_Add` (`self.Triangles`) (+ (`self.YSize`) 2 (`local.Vertext`)))
      (`KismetArrayLibrary.Array_Add` (`self.Triangles`) (+ (`self.YSize`) 1 (`local.Vertext`)))
      (`/Engine/EditorBlueprintResources/StandardMacros.IncrementInt` (`local.Vertext`)))
    (`/Engine/EditorBlueprintResources/StandardMacros.IncrementInt` (`local.Vertext`))))

(fn `Generate Verticies`
  (locals (X :type Integer) (Y :type Integer))
  (bind _scale (`self.Scale`))
  (bind _scale_2 (`self.Scale`))
  (bind _scale_3 (`self.Scale`))
  (for _index (range (+ (`self.XSize`) 1))
    (set `local.X` _index)
    (for _index_2 (range (+ (`self.YSize`) 1))
      (set `local.Y` _index_2)
      (`KismetArrayLibrary.Array_Add` (`self.Vertices`) (`KismetMathLibrary.MakeVector` (* (`local.X`) _scale) (* (`local.Y`) _scale) (`KismetMathLibrary.RandomFloatInRange` (`self.ZMin`) (`self.ZMax`))))
      (`KismetArrayLibrary.Array_Add` (`self.UV0`) (`KismetMathLibrary.MakeVector2D` (* (`local.X`) _scale_2) (* (`local.Y`) _scale_2)))
      (`KismetSystemLibrary.DrawDebugSphere` (`KismetMathLibrary.MakeVector` (* (`local.X`) _scale_3) (* (`local.Y`) _scale_3)) 25.0 12 (struct :`R` 1.0 :`B` 0.017848 :`A` 1.0) 999.0))))

(fn `UserConstructionScript`)